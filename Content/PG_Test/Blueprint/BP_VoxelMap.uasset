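; BP_VoxelMap generates a grid map of ground, food, wood and stone tiles as instanced static meshes.
; GenerateGrid optionally randomizes the noise offset, clears all instances, then places one per cell.
; Summed steep and smooth terrain-height samples are compared to water, food and stone levels to pick each cell's mesh.
; Computed height only selects the mesh, as every instance shares WaterLevel as its Z scale.
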(event `DestroyGrid`
  (`InstancedStaticMeshComponent.ClearInstances` (`self.ISM_Food`))
  (`InstancedStaticMeshComponent.ClearInstances` (`self.ISM_Stone`))
  (`InstancedStaticMeshComponent.ClearInstances` (`self.ISM_Wood`))
  (`InstancedStaticMeshComponent.ClearInstances` (`self.ISM_Ground`)))

(event `GenerateGrid`
  (bind _returnvalue (* (`KismetMathLibrary.RandomFloat`) 5000000000.0))
  (bind _returnvalue_2 (- (`KismetMathLibrary.Conv_IntToDouble` (/ (`self.GridSize`) (`self.VoxelSize`))) 0.05))
  (if (`self.RandomLayout`)
    (set `self.PerlinOffset` (`KismetMathLibrary.MakeVector2D` _returnvalue _returnvalue)))
  (`self.DestroyGrid`)
  (for _index (range (+ (`self.YCount`) 1))
    (for _index_2 (range (+ (`self.XCount`) 1))
      (bind _returnvalue_3 (+ (* (`KismetMathLibrary.MakeVector` (`KismetMathLibrary.Conv_IntToDouble` _index_2) (`KismetMathLibrary.Conv_IntToDouble` _index)) (`self.GridSize`)) (`self.K2_GetActorLocation`)))
      (`InstancedStaticMeshComponent.AddInstance` (`.ISM` (`self.GetHeight` _returnvalue_3)) (`KismetMathLibrary.MakeTransform` _returnvalue_3 (struct) (`KismetMathLibrary.MakeVector` _returnvalue_2 _returnvalue_2 (`self.WaterLevel`))) true))))

(fn `GetHeight`
  (params (InVector :type "Vector Structure"))
  (returns (ReturnValue :type "Float (double-precision)") (ISM :type "InstancedStaticMeshComponent Object Reference"))
  (locals (z :type "Float (double-precision)"))
  (bind _waterlevel (`self.WaterLevel`))
  (bind _returnvalue (+ (`KismetMathLibrary.Conv_VectorToVector2D` InVector) (`self.PerlinOffset`)))
  (bind _returnvalue_2 (`self.GetTerrainHeight` _returnvalue (`self.Steep Scale`) (`self.Steep Amplitude`)))
  (bind _returnvalue_3 (`self.GetTerrainHeight` _returnvalue (`self.Smooth Scale`) (`self.Smooth Amplitude`)))
  (set `local.z` (`KismetMathLibrary.FMax` (/ (+ _returnvalue_2 _returnvalue_3) (`self.VoxelSize`)) 1.0))
  (if (== (`local.z`) (`self.WaterLevel`))
    (return (`self.WaterLevel`) (`self.ISM_Ground`))
    (elif (`KismetMathLibrary.InRange_FloatFloat` (`local.z`) _waterlevel (+ _waterlevel (`self.FoodLevel`)))
      (return (+ (`self.WaterLevel`) 1.0) (`self.ISM_Food`))
      (else
        (set `local.z` (+ (- (`local.z`) (`self.FoodLevel`)) (`self.WaterLevel`)))
        (return (`local.z`) (select `bool` (> (`local.z`) (`self.StoneLevel`)) :`false` (`self.ISM_Wood`) :`true` (`self.ISM_Stone`)))))))

(fn `UserConstructionScript`)