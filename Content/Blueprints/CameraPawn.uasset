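; CameraPawn is a pawn that places buildings on a grid where the player clicks.
; A left click traces a line from the mouse cursor into the world to get an impact point.
; It then searches the first GridActor's GridArray for the location closest to that point, within a fixed maximum distance.
; When a valid location is found, it spawns a BP_Building01 there, without checking whether the spot is occupied.
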(event `Key|LeftMouseButton`
  (params (Key :type "Key Structure"))
  (bind (_worldlocation _worlddirection) (`PlayerController.DeprojectMousePositionToWorld` (`GameplayStatics.GetPlayerController` 0)))
  (bind _gridarray (`/Game/Blueprints/Buildings/GridPlacement/GridActor.GridArray` (`self.Grid Reference`)))
  ;[0.324 1 0.3655] On Click, Get the Mouse Location in the World, Draw a Line to It
  (:`Pressed`
    (bind (_outhit _returnvalue) (`KismetSystemLibrary.LineTraceSingle` :`Start` _worldlocation :`End` (+ _worldlocation (* _worlddirection 1000000.0)) :`TraceChannel` "TraceTypeQuery3" :`DrawTime` 1.0))
    (if _returnvalue
      (set `self.Impact Point` (`.ImpactPoint` (`GameplayStatics.BreakHitResult` _outhit)))
      ;[0.4799 0.5036 1] Find Each Build Actor, Add them to an Array, Reset Closest Distance
      (bind _outactors (`GameplayStatics.GetAllActorsOfClass` "/Game/Blueprints/Buildings/GridPlacement/GridActor.GridActor_C"))
      (set `self.Grid Reference` (`|GetArrayItem` _outactors))
      (set `self.ClosestDistance` 500.0)
      ;[1 1 1] Find the Closest Location to the Hit Point
      (set `self.ValidLocation` false)
      (for (_array_element _array_index) _gridarray
        (bind _returnvalue_2 (`KismetMathLibrary.Vector_Distance` _array_element (`self.Impact Point`)))
        (if (< _returnvalue_2 (`self.ClosestDistance`))
          (set `self.ClosestDistance` _returnvalue_2)
          (set `self.ClosestGridLocation` (`|GetArrayItem` _gridarray _array_index))
          (set `self.ValidLocation` true)))
      ;[1 0.2972 0.4375] If a Valid Location is Found, place a building there
      (if (`self.ValidLocation`)
        (`|SpawnActorFromClass` "/Game/Blueprints/Buildings/BP_Building01.BP_Building01_C" (`KismetMathLibrary.MakeTransform` (`self.ClosestGridLocation`)) "Undefined" "MultiplyWithRoot" null null)))))

(fn `UserConstructionScript`)